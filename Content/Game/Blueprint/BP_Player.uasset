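; Player pawn for a board game that hops tile by tile along BP_Board by the number BP_Dice rolls.
; MoveBy takes signed steps, then recursive StepForward asks the board for each next index, moves the capsule there and calls Land on the final tile.
; The tile index is saved every step and restored on BeginPlay; X deletes the save.
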(event Custom|OnDiceRoll
  (params (Result :type Integer))
  ;[0.2014 0.3706 1] joueur écoute l'info envoyé par BP_Dice (résultat) et le reprend pour savoir de combien doit avancer => déclenche fonction move by
  (CallFunction|Moveby Result))

(event Custom|Move%20By
  (params (Steps :type Integer))
  ;[1 0.9176 0.1725] c'est la fonction qui va permettre de faire avancer (ou reculer) le joueur. Si true = player pas en mouvement donc peut avancer mouvement donc pas possible de lancer le dé.
  (if (not (Variables|Default|GetIsMoving))
    (Variables|Default|SetIsMoving true)
    (if (!= Steps 0)
      (Variables|Default|SetDirection (Class|KismetMathLibrary|SignOfInteger Steps))
      (Variables|Default|SetIsMoving true)
      (Utilities|FlowControl|Delay 0.6)
      (CallFunction|StepForward (Math|Integer|Absolute(Integer) Steps)))))

(event Custom|StepForward
  (params (Remaining :type Integer))
  ;[1 0.9176 0.1725] Si il reste des pas à faire (=> remaining > supèrieur à 0) alors le pion va demander au board l'index la case ou aller et aller dessus (move component to) sa position va etre save et ainsi de suite jusq'à ce que remaining = 0
  (if (> Remaining 0)
    (bind _result (Default|NextIndex (Variables|Default|GetBoard) (Variables|Default|GetCurrentIndex) (Variables|Default|GetDirection)))
    (Variables|Default|SetCurrentIndex _result)
    (Components|MoveComponentTo (Variables|Collision|GetCapsuleComponent) (+ (Transformation|GetActorLocation (Utilities|Array|Get(acopy) (Variables|/Game/Game/Blueprint/BP_Board.BP_Board_C|GetTiles (Variables|Default|GetBoard)) (Variables|Default|GetCurrentIndex))) "0.000000,0.000000,100.000000") "0, 0, 0" false false 0.3 false)
    (CallFunction|SavePosition)
    (Utilities|FlowControl|Delay 0.5)
    (CallFunction|StepForward (- Remaining 1))
    (else
      (Variables|Default|SetIsMoving false)
      (Default|Land (Utilities|Array|Get(acopy) (Variables|/Game/Game/Blueprint/BP_Board.BP_Board_C|GetTiles (Variables|Default|GetBoard)) (Variables|Default|GetCurrentIndex)) self))))

(event Custom|SavePosition
  ;[0.6275 0.2275 1] Système de Save de la position du joueur mémorise l'index de la case sur laquel il est
  (bind _returnvalue (SaveGame|CreateSaveGameObject "/Game/Game/Blueprint/BP_SaveData.BP_SaveData_C"))
  (Variables|/Game/Game/Blueprint/BP_SaveData.BP_SaveData_C|SetSaveIndex _returnvalue (Variables|Default|GetCurrentIndex))
  (SaveGame|SaveGametoSlot _returnvalue "OieGameSave"))

(event EventBeginPlay
  (bind _returnvalue (Actor|GetActorOfClass "/Game/Game/Blueprint/BP_Board.BP_Board_C"))
  (Variables|Default|SetBoard _returnvalue)
  (bind _returnvalue_2 (Actor|GetActorOfClass "/Game/Game/Blueprint/BP_Dice.BP_Dice_C"))
  ;[0.2014 0.3706 1] joueur écoute l'info envoyé par BP_Dice (résultat) et le reprend pour savoir de combien doit avancer => déclenche fonction move by
  (EventDispatchers|BindEventtoOnRolled _returnvalue_2 (delegate Custom|OnDiceRoll))
  ;[0.6275 0.2275 1] charge la sauvegarde de l'index de la case sur laquel était le joueur. Si il y a une sauvegarde alors elle se charge et positionne le joueur a l'index correpondant
  (Utilities|FlowControl|Delay 0.1)
  (bind _returnvalue_3 (SaveGame|DoesSaveGameExist "OieGameSave"))
  (if _returnvalue_3
    (bind _returnvalue_4 (SaveGame|LoadGamefromSlot "OieGameSave"))
    (bind _asbp_save_data (Utilities|Casting|CastToBP_SaveData _returnvalue_4))
    (Variables|Default|SetCurrentIndex (Variables|/Game/Game/Blueprint/BP_SaveData.BP_SaveData_C|GetSaveIndex _asbp_save_data))
    (Transformation|SetActorLocation (+ (Transformation|GetActorLocation (Utilities|Array|Get(acopy) (Variables|/Game/Game/Blueprint/BP_Board.BP_Board_C|GetTiles (Variables|Default|GetBoard)) (Variables|Default|GetCurrentIndex))) "0.000000,0.000000,100.000000") false false)))

(event Input|KeyboardEvents|X
  (params (Key :type Key%20Structure :default "None"))
  ;[0.6275 0.2275 1] permet de supprimer la save de la position du joueur et reprendre à la case initial (se mettra à jour en relancant le jeu)
  (:Pressed
    (SaveGame|DeleteGameinSlot "OieGameSave")))

(fn ConstructionScript)