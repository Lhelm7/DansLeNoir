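; BP_Board is the game board, keeping an ordered, looping track of the BP_Tile actors in the level.
; On BeginPlay it gathers every tile and stores it in the Tiles array at the index given by its Number.
; NextIndex offsets an index by Direction and uses modulo on the tile count to wrap around the board.
; GenerateBoard, GetTile and GetCenterTile are inert stubs, with leftover unconnected grid logic.
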(event EventBeginPlay
  ;[1 1 1] création de la liste des tiles, on récupère tous les acteurs et on les range en fonction de leur index = number (numéro à mettre dans l'inspector)
  (bind _outactors (Actor|GetAllActorsOfClass "/Game/Game/Blueprint/BP_Tile.BP_Tile_C"))
  (for _array_element _outactors
    (bind _asbp_tile (Utilities|Casting|CastToBP_Tile _array_element))
    (Utilities|Array|SetArrayElem (Variables|Default|GetTiles) (Variables|/Game/Game/Blueprint/BP_Tile.BP_Tile_C|GetNumber _asbp_tile) _asbp_tile true)))

(event Collision|EventActorBeginOverlap
  (params (OtherActor :type Actor%20Object%20Reference)))

(event EventTick
  (params (DeltaSeconds :type Float%20%28single-precision%29)))

(fn ConstructionScript)

(fn GenerateBoard)

(fn GetTile
  (params (Coords :type Int%20Point%20Structure)))

(fn GetCenterTile)

(fn NextIndex
  (params (Index :type Integer) (Direction :type Integer))
  (bind _tiles (Variables|Default|GetTiles))
  (bind _returnvalue (Utilities|Array|Length _tiles))
  ;[1 1 1] calcul par rapport à l'index des tiles dans le tableau (ajoute +1 au jet) et le modulo permet de faire boucler le plateau
  (return (Math|Integer|%(Integer) (+ Index Direction _returnvalue) _returnvalue)))