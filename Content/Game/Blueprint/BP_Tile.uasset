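; BP_Tile is a board game tile that shows its number and can apply a bonus or penalty move to a pawn that lands on it.
; The construction script writes Number into the Name text component.
; Land, intended for when a pawn finishes moving, calls the OnPlayerLanded dispatcher, then calls the player's MoveBy with BonusSteps if that value is nonzero.
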(event EventBeginPlay)

(event Collision|EventActorBeginOverlap
  (params (OtherActor :type Actor%20Object%20Reference)))

(event EventTick
  (params (DeltaSeconds :type Float%20%28single-precision%29)))

(fn ConstructionScript
  (Rendering|Components|TextRender|SetText (Variables|Default|GetName) (Utilities|Text|ToText(Integer) (Variables|Default|GetNumber))))

(fn Land
  (params (Player :type BP%20Player%20Object%20Reference))
  ;[1 1 1] Event quand le pion à fini son déplacement si il se trouve sur une case avec bonus steps différents de 0 (+2/-3) alors ca relance la fonction move by mais en prenant en compte le bonus steps
  (Default|CallOnPlayerLanded Player)
  (if (!= (Variables|Default|GetBonusSteps) 0)
    (Default|Moveby Player (Variables|Default|GetBonusSteps))))